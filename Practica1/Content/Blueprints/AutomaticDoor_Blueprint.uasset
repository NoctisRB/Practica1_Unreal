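; Automatic sliding door with upper and lower panels that part vertically when an actor overlaps it and close when one leaves.
; BeginPlay caches each panel's starting world Z, and the overlap events toggle Open and Close flags.
; Tick moves both panels in opposite directions at MovementSpeed until they pass OpenZDelta or their start heights, without sweep or snapping to the exact limit.
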(event EventBeginPlay
  ;[1 1 1] Setting de las posiciones iniciales de las puertas.
  (Variables|OpenDoor|SetupperStartZPos (.Z (Math|Vector|BreakVector (Transformation|GetWorldLocation (Variables|Default|GetUpperDoor)))))
  (Variables|OpenDoor|SetlowerStartZPos (.Z (Math|Vector|BreakVector (Transformation|GetWorldLocation (Variables|Default|GetLowerDoor))))))

(event Collision|EventActorBeginOverlap
  (params (OtherActor :type Actor%20Object%20Reference))
  ;[1 1 1] Eventos de Entrada/Salida
  (Development|PrintString "Entered Door Area")
  (Variables|Default|Setopen true)
  (Variables|Default|Setclose false))

(event EventTick
  (params (DeltaSeconds :type Float%20%28single-precision%29))
  (bind _movementspeed (Variables|OpenDoor|GetmovementSpeed))
  (bind _movementspeed_2 (Variables|OpenDoor|GetmovementSpeed))
  (bind _returnvalue (* DeltaSeconds _movementspeed))
  (bind _returnvalue_2 (* DeltaSeconds _movementspeed_2))
  (if (Variables|Default|Getopen)
    ;[1 1 1] Comprovación de límites
    (if (and (< (.Z (Math|Vector|BreakVector (Transformation|GetWorldLocation (Variables|Default|GetUpperDoor)))) (+ (Variables|OpenDoor|GetupperStartZPos) (Variables|OpenDoor|GetopenZDelta))) (< (- (Variables|OpenDoor|GetlowerStartZPos) (Variables|OpenDoor|GetopenZDelta)) (.Z (Math|Vector|BreakVector (Transformation|GetWorldLocation (Variables|Default|GetLowerDoor))))))
      ;[1 1 1] Movimiento Apertura
      (Transformation|AddRelativeLocation (Variables|Default|GetUpperDoor) (* (Math|Vector|VectorUp) _returnvalue_2) false false)
      (Transformation|AddRelativeLocation (Variables|Default|GetLowerDoor) (* (Math|Vector|VectorDown) _returnvalue_2) false false)
      (else
        (Variables|Default|Setopen false)))
    (elif (Variables|Default|Getclose)
      ;[1 1 1] Comprobación de límites
      (if (and (< (Variables|OpenDoor|GetupperStartZPos) (.Z (Math|Vector|BreakVector (Transformation|GetWorldLocation (Variables|Default|GetUpperDoor))))) (< (.Z (Math|Vector|BreakVector (Transformation|GetWorldLocation (Variables|Default|GetLowerDoor)))) (Variables|OpenDoor|GetlowerStartZPos)))
        ;[1 1 1] Movimiento de cerrar
        (Transformation|AddRelativeLocation (Variables|Default|GetUpperDoor) (* (Math|Vector|VectorDown) _returnvalue) false false)
        (Transformation|AddRelativeLocation (Variables|Default|GetLowerDoor) (* (Math|Vector|VectorUp) _returnvalue) false false)
        (else
          (Variables|Default|Setclose false))))))

(event Collision|EventActorEndOverlap
  (params (OtherActor :type Actor%20Object%20Reference))
  ;[1 1 1] Eventos de Entrada/Salida
  (Development|PrintString "Exited Door Area")
  (Variables|Default|Setclose true)
  (Variables|Default|Setopen false))

(fn ConstructionScript)