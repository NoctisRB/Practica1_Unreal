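; PuzzleLight is a point light Blueprint for a puzzle whose color the player can change.
; On BeginPlay it applies the color at LightIndex from ColorArray.
; A trigger overlap toggles CanBeChanged, so pressing E inside it picks a random color.
; The random pick rerolls until it differs from the current index, then stores it as the new LightIndex.
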(event OnComponentBeginOverlap(LightTrigger_1)
  (params (OverlappedComponent :type Primitive%20Component%20Object%20Reference) (OtherActor :type Actor%20Object%20Reference) (OtherComp :type Primitive%20Component%20Object%20Reference) (OtherBodyIndex :type Integer) (bFromSweep :type Boolean) (SweepResult :type Hit%20Result%20Structure%20%28by%20ref%29))
  (Variables|Default|SetcanBeChanged true))

(event OnComponentEndOverlap(LightTrigger_1)
  (params (OverlappedComponent :type Primitive%20Component%20Object%20Reference) (OtherActor :type Actor%20Object%20Reference) (OtherComp :type Primitive%20Component%20Object%20Reference) (OtherBodyIndex :type Integer))
  (Variables|Default|SetcanBeChanged false))

(event EventBeginPlay
  (CallFunction|ChangeColor))

(event EventTick
  (params (DeltaSeconds :type Float%20%28single-precision%29)))

(event Input|KeyboardEvents|E
  (params (Key :type Key%20Structure :default "None"))
  (:Pressed
    (if (Variables|Default|GetcanBeChanged)
      (CallFunction|ChangeRandomColor))))

(fn ConstructionScript)

(fn ChangeColor
  (Rendering|Components|Light|SetLightColor (Variables|Default|GetPointLightComponent) (Math|Conversions|ToLinearColor(Color) (Utilities|Array|Get(acopy) (Variables|Default|GetcolorArray) (Variables|Default|GetlightIndex))) true))

(fn GetRandomLight
  (params (maxNumber :type Integer))
  (return (Math|Random|RandomInteger maxNumber)))

(fn ChangeRandomColor
  (bind _colorarray (Variables|Default|GetcolorArray))
  (bind _returnvalue (Utilities|Array|Length _colorarray))
  (bind _number (CallFunction|GetRandomLight _returnvalue))
  (bind _output_get (Variables|ChangeColor|SetrandomNumber _number))
  (while (== (Variables|ChangeColor|GetrandomNumber) (Variables|Default|GetlightIndex))
    (bind _number_2 (CallFunction|GetRandomLight _returnvalue))
    (Variables|ChangeColor|SetrandomNumber _number_2))
  (Rendering|Components|Light|SetLightColor (Variables|Default|GetPointLightComponent) (Math|Conversions|ToLinearColor(Color) (Utilities|Array|Get(acopy) _colorarray _output_get)) true)
  (Variables|Default|SetlightIndex _output_get))