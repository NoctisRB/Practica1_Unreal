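; A door that stays locked until the player has enough coins to pay its opening cost, shown on its info text.
; On overlap it reads the coin count from the game instance's GameData, subtracts the cost if affordable and marks itself unlocked.
; The parent overlap logic runs only once unlocked, so later overlaps pass through without charging again.
; The overlapping actor is not checked.
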(event EventBeginPlay
  (Rendering|Components|TextRender|SetText (Variables|Default|GetInfoText) (Utilities|Text|ToText(String) (Utilities|String|Append (Utilities|String|ToString(Integer) (Variables|Conditions|GetcoinsToOpen)) " Coins")))
  (|CallParentFunction))

(event Collision|EventActorBeginOverlap
  (params (OtherActor :type Actor%20Object%20Reference))
  (bind _coinstoopen (Variables|Conditions|GetcoinsToOpen))
  (if (Variables|Default|Getunlocked)
    _
    (else
      (bind _asgame_instance_blueprint (Utilities|Casting|CastToGameInstance_Blueprint (Game|GetGameInstance)))
      (Math|Integer|CompareInt (.coinsQuantity (Utilities|Struct|BreakGameData (Variables|/Game/Blueprints/GameInstance_Blueprint.GameInstance_Blueprint_C|GetgameData _asgame_instance_blueprint))) _coinstoopen
        (:>
          _)
        (:==
          _))
      (Default|SubstractItems _asgame_instance_blueprint "NewEnumerator1" _coinstoopen)
      (Variables|Default|Setunlocked true)))
  (|CallParentFunction 0))

(event EventTick
  (params (DeltaSeconds :type Float%20%28single-precision%29))
  (|CallParentFunction DeltaSeconds) ; This node is disabled and will not be called.\nDrag off pins to build functionality.
)

(fn ConstructionScript
  (|CallParentFunction))