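; PuzzleDoor_Blueprint is a door that responds to overlaps only when its three-light puzzle is solved.
; On BeginPlay it casts three child actor components to PuzzleLight_Blueprint and stores the references.
; On overlap it compares each light's LightIndex with the door's matching target index, passing the event to the parent class only if all three match.
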(event EventBeginPlay
  ;[1 1 1] Inicializa las variables que referencian los blueprints de las luces hijas
  (|CallParentFunction)
  (bind _aspuzzle_light_blueprint (Utilities|Casting|CastToPuzzleLight_Blueprint (Variables|/Script/Engine.ChildActorComponent|GetChildActor (Variables|Default|GetPuzzleLight_Blueprint_1))))
  (Variables|Default|Setlight1_BP _aspuzzle_light_blueprint)
  (bind _aspuzzle_light_blueprint_2 (Utilities|Casting|CastToPuzzleLight_Blueprint (Variables|/Script/Engine.ChildActorComponent|GetChildActor (Variables|Default|GetPuzzleLight_Blueprint_2))))
  (Variables|Default|Setlight2_BP _aspuzzle_light_blueprint_2)
  (bind _aspuzzle_light_blueprint_3 (Utilities|Casting|CastToPuzzleLight_Blueprint (Variables|/Script/Engine.ChildActorComponent|GetChildActor (Variables|Default|GetPuzzleLight_Blueprint_3))))
  (Variables|Default|Setlight3_BP _aspuzzle_light_blueprint_3))

(event EventTick
  (params (DeltaSeconds :type Float%20%28single-precision%29))
  (|CallParentFunction DeltaSeconds))

(event EventActorBeginOverlap
  (params (OtherActor :type Actor%20Object%20Reference))
  ;[1 1 1] Comprueba que las 3 luces sean las correctas
  (if (Math|Boolean|ANDBoolean (== (Variables|/Game/Blueprints/Doors/PuzzleLight_Blueprint.PuzzleLight_Blueprint_C|GetlightIndex (Variables|Default|Getlight1_BP)) (Variables|Indexes|GetlightIndex1)) (== (Variables|/Game/Blueprints/Doors/PuzzleLight_Blueprint.PuzzleLight_Blueprint_C|GetlightIndex (Variables|Default|Getlight2_BP)) (Variables|Indexes|GetlightIndex2)) (== (Variables|/Game/Blueprints/Doors/PuzzleLight_Blueprint.PuzzleLight_Blueprint_C|GetlightIndex (Variables|Default|Getlight3_BP)) (Variables|Indexes|GetlightIndex3)))
    (|CallParentFunction OtherActor)))

(fn ConstructionScript
  (|CallParentFunction))