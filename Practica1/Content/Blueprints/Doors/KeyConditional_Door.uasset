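; Key-locked door Blueprint that shows how many keys it needs and unlocks when the game's key count is high enough.
; On BeginPlay it writes the required count to its InfoText.
; On any actor overlap while locked, it checks the GameInstance key count, subtracts the cost and sets Unlocked.
; Once unlocked, overlaps pass to the parent class's overlap handler; too few keys leaves that handler uncalled.
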(event EventBeginPlay
  ;[1 1 1] Pone el valor en el texto de la puerta
  (Rendering|Components|TextRender|SetText (Variables|Default|GetInfoText) (Utilities|Text|ToText(String) (Utilities|String|Append (Utilities|String|ToString(Integer) (Variables|Default|GetkeysToOpen)) " Keys")))
  (|CallParentFunction))

(event Collision|EventActorBeginOverlap
  (params (OtherActor :type Actor%20Object%20Reference))
  (bind _keystoopen (Variables|Default|GetkeysToOpen))
  ;[1 1 1] Comprueba que haya el número de llaves indicado y desbloquea la puerta
  (if (Variables|Default|Getunlocked)
    _
    (else
      (bind _asgame_instance_blueprint (Utilities|Casting|CastToGameInstance_Blueprint (Game|GetGameInstance)))
      (Math|Integer|CompareInt (.keysQuantity (Utilities|Struct|BreakGameData (Variables|/Game/Blueprints/GameInstance_Blueprint.GameInstance_Blueprint_C|GetgameData _asgame_instance_blueprint))) _keystoopen
        (:>
          _)
        (:==
          _))
      (Default|SubstractItems _asgame_instance_blueprint "NewEnumerator0" _keystoopen)
      (Variables|Default|Setunlocked true)))
  (|CallParentFunction OtherActor))

(event EventTick
  (params (DeltaSeconds :type Float%20%28single-precision%29))
  (|CallParentFunction DeltaSeconds) ; This node is disabled and will not be called.\nDrag off pins to build functionality.
)

(fn ConstructionScript
  (|CallParentFunction))