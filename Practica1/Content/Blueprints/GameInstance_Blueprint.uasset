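; Game instance Blueprint that tracks the player's key and coin counts and reflects them in the level UI.
; AddItem switches on item type, increments the matching count in GameData, updates its LevelUI text, then prints the coin count.
; SubstractItems displays the count minus the given quantity in LevelUI, but does not write the reduced value back to GameData.
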(event EventAddItem
  (params (itemType :type ItemType%20Enum :default "NewEnumerator0"))
  (bind _gamedata (Variables|Default|GetgameData))
  (bind _levelui (Variables|Default|GetLevelUI))
  (bind (_coinsquantity _keysquantity) (Utilities|Struct|BreakGameData _gamedata))
  ;[1 1 1] Adds an item of the indicated type
  (switch Utilities|FlowControl|Switch|SwitchonItemType itemType
    (:NewEnumerator0
      (bind _result (Math|Integer|IncrementInt _keysquantity)
        (:%20%20
          (Default|SetKeyText _levelui _result))))
    (:NewEnumerator1
      (bind _result_2 (Math|Integer|IncrementInt _coinsquantity)
        (:%20%20
          (Default|SetCoinText _levelui _result_2)))))
  (Development|PrintString (Utilities|String|ToString(Integer) _coinsquantity)))

(fn SubstractItems
  (params (itemType :type ItemType%20Enum :default "NewEnumerator0") (quantity :type Integer))
  (bind _gamedata (Variables|Default|GetgameData))
  (bind _levelui (Variables|Default|GetLevelUI))
  (bind (_coinsquantity _keysquantity) (Utilities|Struct|BreakGameData _gamedata))
  (switch Utilities|FlowControl|Switch|SwitchonItemType itemType
    (:NewEnumerator0
      (Default|SetKeyText _levelui (- _keysquantity quantity)))
    (:NewEnumerator1
      (Default|SetCoinText _levelui (- _coinsquantity quantity)))))