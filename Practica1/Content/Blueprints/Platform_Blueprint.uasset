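; Platform actor that bobs up and down continuously along the Z axis.
; Each Tick adds the sine of its time since creation, scaled by the Factor variable, to its current Z, keeping X, Y, rotation and scale.
; The offset accumulates per frame without delta time, so travel distance depends on frame rate.
; The move is not swept; BeginPlay, overlap and construction logic are empty.
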(event EventBeginPlay)

(event Collision|EventActorBeginOverlap
  (params (OtherActor :type Actor%20Object%20Reference)))

(event EventTick
  (params (DeltaSeconds :type Float%20%28single-precision%29))
  (bind _returnvalue (Transformation|GetActorTransform))
  (bind (_location _rotation _scale) (Math|Transform|BreakTransform _returnvalue))
  (bind (_x _y _z) (Math|Vector|BreakVector _location))
  (Transformation|SetActorTransform (Math|Transform|MakeTransform (Math|Vector|MakeVector _x _y (+ (* (Math|Trig|Sin(Radians) (Actor|GetGameTimeSinceCreation)) (Variables|Default|Getfactor)) _z)) _rotation _scale)))

(fn ConstructionScript)