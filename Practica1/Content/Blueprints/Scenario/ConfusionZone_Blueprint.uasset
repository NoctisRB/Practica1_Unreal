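; ConfusionZone_Blueprint is a trigger actor that temporarily confuses a ThirdPersonCharacter entering it.
; On overlap it sets the character's Confused flag, stores the character and resets a timer.
; Tick accumulates time and clears the flag once TimeToStopConfusion is reached, whether or not the character has left.
; It tracks only one affected character, so a new overlap replaces the stored one and restarts the countdown.
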(event EventBeginPlay)

(event Collision|EventActorBeginOverlap
  (params (OtherActor :type Actor%20Object%20Reference))
  ;[1 1 1] Set Confusion
  (bind _asthird_person_character (Utilities|Casting|CastToThirdPersonCharacter OtherActor))
  (Variables|/Game/Blueprints/ThirdPersonBP/ThirdPersonCharacter.ThirdPersonCharacter_C|SetConfused _asthird_person_character true)
  (Variables|Default|SetcharacterAffected _asthird_person_character)
  (Variables|Default|SetplayerConfused true)
  (Variables|Default|Settimer 0.0))

(event EventTick
  (params (DeltaSeconds :type Float%20%28single-precision%29))
  ;[1 1 1] Timer to End Confusion
  (if (Variables|Default|GetplayerConfused)
    (bind _output_get (Variables|Default|Settimer (+ (Variables|Default|Gettimer) DeltaSeconds)))
    (Math|Float|CompareFloat _output_get (Variables|Default|GettimeToStopConfusion)
      (:>
        _)
      (:==
        _))
    (Variables|/Game/Blueprints/ThirdPersonBP/ThirdPersonCharacter.ThirdPersonCharacter_C|SetConfused (Variables|Default|GetcharacterAffected) false)
    (Variables|Default|SetplayerConfused false)))

(fn ConstructionScript)