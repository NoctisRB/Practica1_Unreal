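; SaveGameClass is a save game object that holds SavedGameData and handles its own saving, loading and deletion by slot.
; SaveObject writes the object itself to the given slot and user index.
; LoadObject checks that the slot exists, casts the loaded save, copies its SavedGameData into this instance and returns whether it existed.
; DeleteObject removes a named slot, always for user index zero.
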(fn SaveObject
  (params (SlotName :type String) (UserIndex :type Integer))
  (SaveGame|SaveGametoSlot self SlotName UserIndex)
  (return))

(fn LoadObject
  (params (SlotName :type String) (UserIndex :type Integer))
  (bind _returnvalue (SaveGame|DoesSaveGameExist SlotName UserIndex))
  (if _returnvalue
    (bind _returnvalue_2 (SaveGame|LoadGamefromSlot SlotName UserIndex))
    (bind _assave_game_class (Utilities|Casting|CastToSaveGameClass _returnvalue_2))
    (Variables|Default|SetSaved%20Game%20Data (Variables|SaveGameClass_C|GetSaved%20Game%20Data _assave_game_class)))
  (return _returnvalue))

(fn DeleteObject
  (params (SlotName :type String))
  (SaveGame|DeleteGameinSlot SlotName))