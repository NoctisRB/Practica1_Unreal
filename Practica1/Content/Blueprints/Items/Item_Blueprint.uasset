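; Pickup item actor that gives its ItemType to the player's FirstPersonCharacter on overlap, then destroys itself.
; Any overlap triggers the pickup, since it uses player pawn 0 without checking the overlapping actor.
; Before destruction it flags itself Destroyed and calls the game instance's Save.
; Its Save event records its display name in DestroyedObjects, and Load destroys it if that name is listed.
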(event EventBeginPlay)

(event Collision|EventActorBeginOverlap
  (params (OtherActor :type Actor%20Object%20Reference))
  (bind _asfirst_person_character (Utilities|Casting|CastToFirstPersonCharacter (Game|Player|GetPlayerPawn 0)))
  (Default|AddItem _asfirst_person_character (Variables|Item|GetitemType))
  (bind _asgame_instance_blueprint (Utilities|Casting|CastToGameInstance_Blueprint (Game|GetGameInstance)))
  (Variables|Default|Setdestroyed true)
  (Default|Save _asgame_instance_blueprint)
  (Actor|DestroyActor))

(event EventTick
  (params (DeltaSeconds :type Float%20%28single-precision%29)))

(event EventLoad
  (bind _asgame_instance_blueprint (Utilities|Casting|CastToGameInstance_Blueprint (Game|GetGameInstance)))
  (if (Utilities|Array|ContainsItem (.destroyedObjects (Utilities|Struct|BreakGameData (Variables|/Game/Blueprints/Save/SaveGameClass.SaveGameClass_C|GetSaved%20Game%20Data (Variables|/Game/Blueprints/GameInstance_Blueprint.GameInstance_Blueprint_C|GetSavedGameClass _asgame_instance_blueprint)))) (Utilities|GetDisplayName self))
    (Actor|DestroyActor)))

(event EventSave
  (if (Variables|Default|Getdestroyed)
    (bind _asgame_instance_blueprint (Utilities|Casting|CastToGameInstance_Blueprint (Game|GetGameInstance)))
    (Utilities|Array|Add (.destroyedObjects (Utilities|Struct|BreakGameData (Variables|/Game/Blueprints/Save/SaveGameClass.SaveGameClass_C|GetSaved%20Game%20Data (Variables|/Game/Blueprints/GameInstance_Blueprint.GameInstance_Blueprint_C|GetSavedGameClass _asgame_instance_blueprint)))) (Utilities|GetDisplayName self))))

(fn ConstructionScript)