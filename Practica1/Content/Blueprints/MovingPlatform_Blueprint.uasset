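; Moving platform Blueprint that oscillates the actor vertically along a cosine wave.
; BeginPlay sets the wave's center one Amplitude above the starting Z.
; Tick accumulates a timer and sets Z from Period and Amplitude without sweeping, so motion begins at the cosine peak, two Amplitudes above the placed height.
; X and Y stay unchanged, and the overlap event only calls its parent.
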(event EventBeginPlay
  (|CallParentFunction)
  (Variables|Default|SetcenterZ (+ (.Z (Math|Vector|BreakVector (Transformation|GetActorLocation))) (Variables|Sinus|Getamplitude))))

(event Collision|EventActorBeginOverlap
  (params (OtherActor :type Actor%20Object%20Reference))
  (|CallParentFunction OtherActor) ; This node is disabled and will not be called.\nDrag off pins to build functionality.
)

(event EventTick
  (params (DeltaSeconds :type Float%20%28single-precision%29))
  (bind _returnvalue (Transformation|GetActorLocation))
  (bind (_x _y) (Math|Vector|BreakVector _returnvalue))
  (|CallParentFunction DeltaSeconds)
  (bind _output_get (Variables|Default|Settimer (+ (Variables|Default|Gettimer) DeltaSeconds)))
  (Transformation|SetActorLocation (Math|Vector|MakeVector _x _y (+ (* (Math|Trig|Cos(Radians) (* (/ _output_get (Variables|Sinus|Getperiod)) (* 2 (Math|Trig|GetPI)))) (Variables|Sinus|Getamplitude)) (Variables|Default|GetcenterZ))) false false))

(fn ConstructionScript
  (|CallParentFunction))