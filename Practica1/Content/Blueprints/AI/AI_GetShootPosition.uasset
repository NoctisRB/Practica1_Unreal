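; Behavior Tree task that picks a shooting position for an AI bot relative to the player.
; It takes the point on the line from player 0's pawn toward the bot at the bot's ShootDistance from the player.
; It writes that point to the ShootPosition blackboard key and finishes successfully, with no navmesh or line-of-sight check.
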(event EventReceiveExecuteAI
  (params (OwnerController :type AI%20Controller%20Object%20Reference) (ControlledPawn :type Pawn%20Object%20Reference))
  (bind _returnvalue (Game|Player|GetPlayerPawn 0))
  (bind _returnvalue_2 (Transformation|GetActorLocation _returnvalue))
  (bind _asai_bot_blueprint (Utilities|Casting|CastToAI_BOT_Blueprint ControlledPawn))
  (AI|BehaviorTree|SetBlackboardValueasVector (Variables|Default|GetShootPosition) (+ _returnvalue_2 (* (Math|Vector|Normalize (- (Transformation|GetActorLocation _asai_bot_blueprint) _returnvalue_2)) (Variables|/Game/ThirdPersonBP/Blueprints/AI_BOT_Blueprint.AI_BOT_Blueprint_C|GetShoot%20Distance _asai_bot_blueprint))))
  (AI|BehaviorTree|FinishExecute true))