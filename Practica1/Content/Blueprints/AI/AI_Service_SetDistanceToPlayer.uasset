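; Behavior tree service that updates an AI bot's blackboard with the player's position and its line-of-sight distance to the player.
; Each tick it always writes the player pawn's location, then line traces on the Camera channel from the bot toward that location.
; A first-hit FirstPersonCharacter stores the trace distance; otherwise DistanceToPlayer gets a large fallback equal to the trace length, so an occluded player reads as far away.
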(event EventReceiveTickAI
  (params (OwnerController :type AI%20Controller%20Object%20Reference) (ControlledPawn :type Pawn%20Object%20Reference) (DeltaSeconds :type Float%20%28single-precision%29))
  (bind _returnvalue (Game|GetPlayerController 0))
  (bind _distancetoplayer (Variables|Default|GetDistanceToPlayer))
  (bind _returnvalue_2 (Pawn|GetControlledPawn _returnvalue))
  (bind _returnvalue_3 (Transformation|GetActorLocation _returnvalue_2))
  (bind _asai_bot_blueprint (Utilities|Casting|CastToAI_BOT_Blueprint ControlledPawn))
  (AI|BehaviorTree|SetBlackboardValueasVector (Variables|Default|GetPlayerPosition) _returnvalue_3)
  (bind _outhit (Collision|LineTraceByChannel (Transformation|GetActorLocation _asai_bot_blueprint) (+ (Transformation|GetActorLocation _asai_bot_blueprint) (* (Math|Vector|Normalize (- _returnvalue_3 (Transformation|GetActorLocation _asai_bot_blueprint))) 1e+04)) "TraceTypeQuery2" false (Utilities|Array|MakeArray _asai_bot_blueprint) "None"))
  (Utilities|Casting|CastToFirstPersonCharacter (.HitActor (Collision|BreakHitResult _outhit))
    (:then
      (Class|BTFunctionLibrary|SetBlackboardValueasFloat _distancetoplayer (.Distance (Collision|BreakHitResult _outhit))))
    (:CastFailed
      (Class|BTFunctionLibrary|SetBlackboardValueasFloat _distancetoplayer 1e+04))))